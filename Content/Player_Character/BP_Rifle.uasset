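; BP_Rifle is a player rifle Blueprint that fires a debug hitscan trace on left mouse press.
; The trace runs along the mesh's forward vector on the Visibility channel, draws persistent debug lines and prints the hit actor's name, without applying damage.
; A disconnected physics-impulse and self-destroy chain reads the empty Hit event's component but never runs.
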(event EventBeginPlay)

(event Collision|EventHit
  (params (MyComp :type Primitive%20Component%20Object%20Reference) (Other :type Actor%20Object%20Reference) (OtherComp :type Primitive%20Component%20Object%20Reference) (bSelfMoved :type Boolean) (HitLocation :type Vector :default "0, 0, 0") (HitNormal :type Vector :default "0, 0, 0") (NormalImpulse :type Vector :default "0, 0, 0") (Hit :type Hit%20Result%20Structure%20%28by%20ref%29)))

(event EventTick
  (params (DeltaSeconds :type Float%20%28single-precision%29)))

(event Collision|EventActorBeginOverlap
  (params (OtherActor :type Actor%20Object%20Reference)))

(event Input|MouseEvents|LeftMouseButton
  (params (Key :type Key%20Structure))
  (bind _meshcomp (Variables|Default|GetMeshComp))
  (bind _returnvalue (Transformation|GetWorldLocation _meshcomp))
  (:Pressed
    (bind _outhit (Collision|LineTraceByChannel _returnvalue (+ (* (Math|Vector|GetForwardVector _meshcomp) 5e+03) _returnvalue) "TraceTypeQuery1" false 0 "Persistent"))
    (Development|PrintString (Utilities|GetObjectName (.HitActor (Collision|BreakHitResult _outhit))))))

(fn ConstructionScript)