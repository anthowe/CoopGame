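; BP_Bullet is a bullet actor built around a timed explosion, though the explosion logic is currently disconnected.
; A BeginPlay chain waits briefly, calls Explode, then plays a gunshot sound at the world origin rather than the bullet's location.
; Explode is empty; an unwired chain holds the explosion particles, instigator-credited radial damage, actor destruction and debug sphere showing the damage radius.
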(event Custom|Explode)

(event EventBeginPlay)

(event Collision|EventActorBeginOverlap
  (params (OtherActor :type Actor%20Object%20Reference)))

(event EventTick
  (params (DeltaSeconds :type Float%20%28single-precision%29)))

(event EventBeginPlay
  (:then
    (Utilities|FlowControl|Delay 1.0)
    (CallFunction|Explode)
    (Audio|PlaySoundatLocation "/Game/Core/Gun_Shot-Marvin-1140816320.Gun_Shot-Marvin-1140816320" "0, 0, 0" "0, 0, 0" 1.0 1.0 0.0 0 0 0)))

(fn ConstructionScript)